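; Leva_BP is a one-shot sprite lever that opens its linked Door.
; Overlap with Orbis_BP toggles that character's CanUseAction and the Fase1 in-range flag, and registers the lever on it at entry.
; While in range, Tick polls player 0 for F or gamepad face-left, then swaps sprites from centre to right and sets Done.
; It then calls OpenWithLeva on the door and destroys it after a delay.
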(event `self.ReceiveTick`
  (params (DeltaSeconds :type "Float (single-precision)"))
  (bind _returnvalue (`GameplayStatics.GetPlayerController` 0))
  (bind _door (`self.Door`))
  (if (`self.Done`)
    _
    (elif (`self.Fase1`)
      (if (or (`PlayerController.WasInputKeyJustPressed` _returnvalue "Gamepad_FaceButton_Left") (`PlayerController.WasInputKeyJustPressed` _returnvalue "F"))
        (`PaperSpriteComponent.SetSprite` (`self.RenderComponent`) "/Game/PNG/LevaCentrale.LevaCentrale")
        (`KismetSystemLibrary.Delay` 0.2)
        (`PaperSpriteComponent.SetSprite` (`self.RenderComponent`) "/Game/PNG/LevaDestra.LevaDestra")
        (set `self.Fase1` false)
        (set `self.Done` true)
        (if (`KismetSystemLibrary.IsValid` _door)
          (`DoorComponent.OpenWithLeva` (`/Game/Blueprints/Door_BP.Door` _door))
          (`KismetSystemLibrary.Delay` 6.0)
          (`self.K2_DestroyActor` _door))))))

(event `self.RenderComponent.OnComponentBeginOverlap`
  (params (OverlappedComponent :type "PrimitiveComponent Object Reference") (OtherActor :type "Actor Object Reference") (OtherComp :type "PrimitiveComponent Object Reference") (OtherBodyIndex :type Integer) (bFromSweep :type Boolean) (SweepResult :type "HitResult Structure (by ref)"))
  (bind _asorbis_bp (cast `/Game/Blueprints/Orbis_BP` OtherActor))
  (bind _orbis (`/Game/Blueprints/Orbis_BP.Orbis` _asorbis_bp))
  (set `Orbis.CanUseAction` true _orbis)
  (set `Orbis.Leva` self _orbis)
  (set `self.Fase1` true))

(event `self.RenderComponent.OnComponentEndOverlap`
  (params (OverlappedComponent :type "PrimitiveComponent Object Reference") (OtherActor :type "Actor Object Reference") (OtherComp :type "PrimitiveComponent Object Reference") (OtherBodyIndex :type Integer))
  (bind _asorbis_bp (cast `/Game/Blueprints/Orbis_BP` OtherActor))
  (set `Orbis.CanUseAction` false (`/Game/Blueprints/Orbis_BP.Orbis` _asorbis_bp))
  (set `self.Fase1` false))

(fn `UserConstructionScript`)