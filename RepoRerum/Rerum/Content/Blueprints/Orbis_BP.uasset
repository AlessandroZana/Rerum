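; Orbis_BP is the Blueprint for Orbis, apparently the player character, handling HUD-style values, pausing and input toggling.
; Outside the StartMenu level, Tick converts Orbis fuel levels to fractions and copies dash and jump delays, while the Pause action opens PauseMenu_BP and pauses the game.
; Disable and Enable events toggle player pawn input; Blue and Red events are empty, leaving their sprite-color timelines unconnected.
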(event `self.ReceiveBeginPlay`
  (`self.CastToOrbis` (`self.Orbis`)))

(event `self.ReceiveTick`
  (params (DeltaSeconds :type "Float (single-precision)"))
  (bind _orbis (`self.Orbis`))
  (bind _returnvalue (`GameplayStatics.GetCurrentLevelName` true))
  (if (`KismetStringLibrary.NotEqual_StrStr` _returnvalue "StartMenu")
    (set `self.HeavyFuel%` (`KismetTextLibrary.AsPercent_Float` (/ (`Orbis.heavyFuel` (`self.Orbis`)) 10.0) "FromZero"))
    (set `self.LightFuel%` (`KismetTextLibrary.AsPercent_Float` (/ (`Orbis.lightFuel` (`self.Orbis`)) 200.0) "FromZero"))
    (set `self.dash` (`Orbis.DelayOnDash` _orbis))
    (set `self.jump_0` (`Orbis.DelayOnJump` _orbis))))

(event `InputAction|Pause`
  (params (Key :type "Key Structure" :default "AnyKey"))
  (:`Pressed`
    (bind _returnvalue (`GameplayStatics.GetCurrentLevelName` true))
    (if (`KismetStringLibrary.NotEqual_StrStr` _returnvalue "StartMenu")
      (bind _returnvalue_2 (`|CreateWidget` "/Game/UI/PauseMenu_BP.PauseMenu_BP_C"))
      (`UserWidget.AddToViewport` _returnvalue_2 0)
      (`GameplayStatics.SetGamePaused` true))))

(event `self.Orbis.Blue`)

(event `self.Orbis.Red`)

(event `self.Orbis.Disable`
  (`self.DisableInput` (`GameplayStatics.GetPlayerPawn` 0) (`GameplayStatics.GetPlayerController` 0)))

(event `self.Orbis.Enable`
  (`self.EnableInput` (`GameplayStatics.GetPlayerPawn` 0) (`GameplayStatics.GetPlayerController` 0)))

(fn `UserConstructionScript`)