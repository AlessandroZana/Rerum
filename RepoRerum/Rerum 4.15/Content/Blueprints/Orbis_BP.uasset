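; Orbis_BP is the Blueprint for Orbis, apparently the player character, handling fuel readouts, pausing and death.
; Outside StartMenu, Tick computes heavy and light fuel percentages and mirrors dash and jump delays, while the Pause input opens PauseMenu_BP and pauses the game.
; Overlapping a "death"-tagged actor reloads the level, and Orbis Enable/Disable events toggle player input.
; Blue and Red events are empty, leaving the sprite color timelines unused.
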(event `self.ReceiveBeginPlay`
  (`self.CastToOrbis` (`self.Orbis`))
  (`KismetSystemLibrary.ExecuteConsoleCommand` "disableallscreenmessages"))

(event `self.ReceiveTick`
  (params (DeltaSeconds :type "Float (single-precision)"))
  (bind _orbis (`self.Orbis`))
  (bind _orbis_2 (`self.Orbis`))
  (bind _orbis_3 (`self.Orbis`))
  (bind _returnvalue (`GameplayStatics.GetCurrentLevelName` true))
  (if (`KismetStringLibrary.NotEqual_StrStr` _returnvalue "StartMenu")
    (set `Orbis.heavyfuelpercent` (/ (`Orbis.heavyFuel` _orbis_3) (`Orbis.heavyFuelMax` _orbis_3)) _orbis_3)
    (set `Orbis.lightfuelpercent` (/ (`Orbis.lightFuel` _orbis_2) (`Orbis.lightFuelMax` _orbis_2)) _orbis_2)
    (set `self.dash` (`Orbis.DelayOnDash` _orbis))
    (set `self.jump_0` (`Orbis.DelayOnJump` _orbis))))

(event `InputAction|Pause`
  (params (Key :type "Key Structure" :default "AnyKey"))
  (:`Pressed`
    (bind _returnvalue (`GameplayStatics.GetCurrentLevelName` true))
    (if (`KismetStringLibrary.NotEqual_StrStr` _returnvalue "StartMenu")
      (bind _returnvalue_2 (`|CreateWidget` "/Game/UI/PauseMenu_BP.PauseMenu_BP_C"))
      (`UserWidget.AddToViewport` _returnvalue_2 0)
      (`GameplayStatics.SetGamePaused` true))))

(event `self.Orbis.Blue`)

(event `self.Orbis.Red`)

(event `self.Orbis.Disable`
  (`self.DisableInput` (`GameplayStatics.GetPlayerPawn` 0) (`GameplayStatics.GetPlayerController` 0)))

(event `self.Orbis.Enable`
  (`self.EnableInput` (`GameplayStatics.GetPlayerPawn` 0) (`GameplayStatics.GetPlayerController` 0)))

(event `self.ReceiveActorBeginOverlap`
  (params (OtherActor :type "Actor Object Reference"))
  (if (`self.ActorHasTag` OtherActor "death")
    (bind _returnvalue (`GameplayStatics.GetCurrentLevelName` true))
    (`GameplayStatics.OpenLevel` (`KismetStringLibrary.Conv_StringToName` _returnvalue))))

(fn `UserConstructionScript`)